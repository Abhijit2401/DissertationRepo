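; Player character Blueprint for a dungeon game that connects input and gameplay events to the UI and combat feedback.
; BeginPlay adds the HUD, P opens a pausing menu, Tab shows a menu while held, and H uses a health potion.
; Damage events spawn floating text actors flagged for crit or magic, and death shows a paused defeat screen with UI-only input.
; SetMenuState and UseHealthPotion are called here but implemented outside this graph.
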(event `self.ShowDamageNumber`
  (params (DamageAmount :type "Float (single-precision)") (HitLocation :type "Vector Structure") (bIsCrit :type Boolean) (bIsMagic :type Boolean))
  (`|SpawnActorFromClass` "/Game/BP_DamageTextActor.BP_DamageTextActor_C" (`KismetMathLibrary.MakeTransform` HitLocation) "Undefined" "MultiplyWithRoot" null DamageAmount bIsCrit bIsMagic null))

(event `self.ReceiveBeginPlay`
  (`self.SetMenuState` false)
  (bind _returnvalue (`|CreateWidget` "/Game/WBP_DungeonHUD_v2.WBP_DungeonHUD_v2_C"))
  (`UserWidget.AddToViewport` _returnvalue 0))

(event `Key|P`
  (params (Key :type "Key Structure"))
  (:`Pressed`
    (bind _returnvalue (`|CreateWidget` "/Game/WBP_PauseMenu.WBP_PauseMenu_C"))
    (`UserWidget.AddToViewport` _returnvalue 0)
    (`GameplayStatics.SetGamePaused` true)
    (`self.SetMenuState` true)))

(event `self.OnPlayerDied`
  (bind _returnvalue (`GameplayStatics.GetPlayerController` 0))
  (bind _returnvalue_2 (`|CreateWidget` "/Game/WBP_DefeatScreen.WBP_DefeatScreen_C"))
  (`UserWidget.AddToViewport` _returnvalue_2 0)
  (set `PlayerController.bShowMouseCursor` true _returnvalue)
  (`WidgetBlueprintLibrary.SetInputMode_UIOnlyEx` _returnvalue null)
  (`GameplayStatics.SetGamePaused` true))

(event `Key|H`
  (params (Key :type "Key Structure"))
  (:`Pressed`
    (`self.UseHealthPotion`)))

(event `Key|Tab`
  (params (Key :type "Key Structure"))
  (:`Pressed`
    (bind _returnvalue (`|CreateWidget` "/Game/WBP_TabMenu.WBP_TabMenu_C"))
    (bind _output_get (set `self.ActiveTabMenu` _returnvalue))
    (`UserWidget.AddToViewport` _output_get 0)
    (`self.SetMenuState` true))
  (:`Released`
    (bind _activetabmenu (`self.ActiveTabMenu`)
      (:`then`
        (`Widget.RemoveFromParent` _activetabmenu)
        (`self.SetMenuState` false))
      (:`else`))))

(fn `UserConstructionScript`)