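; BP_Shopkeeper is an interactable shopkeeper that opens a shop UI for the player.
; Interact calls the parent, then creates a WBP_Shop widget, adds it to the viewport and turns on the DungeonCharacter's menu state.
; When a DungeonCharacter leaves the DistanceDetector overlap, any valid shop window is removed and that character's menu state is turned off.
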(event `self.Interact`
  (params (InstigatorPawn :type "Pawn Object Reference"))
  (`parent.Interact` null)
  (bind _returnvalue (`|CreateWidget` "/Game/WBP_Shop.WBP_Shop_C" (`GameplayStatics.GetPlayerController` 0)))
  (bind _output_get (set `self.ActiveShopWindow` _returnvalue))
  (`UserWidget.AddToViewport` _output_get 0)
  (bind _asdungeon_character (cast `DungeonCharacter` (`GameplayStatics.GetPlayerCharacter` 0)))
  (`DungeonCharacter.SetMenuState` _asdungeon_character true))

(event `self.DistanceDetector.OnComponentEndOverlap`
  (params (OverlappedComponent :type "PrimitiveComponent Object Reference") (OtherActor :type "Actor Object Reference") (OtherComp :type "PrimitiveComponent Object Reference") (OtherBodyIndex :type Integer))
  (bind _activeshopwindow (`self.ActiveShopWindow`))
  (bind _asdungeon_character (cast `DungeonCharacter` OtherActor))
  (`/Engine/EditorBlueprintResources/StandardMacros.IsValid` _activeshopwindow
    (:`Is Valid`
      (`Widget.RemoveFromParent` _activeshopwindow)
      (`DungeonCharacter.SetMenuState` _asdungeon_character false))))

(fn `UserConstructionScript`)