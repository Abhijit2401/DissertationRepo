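; BP_DamageTextActor is a floating damage number actor that shows an amount through a WBP_DamageText widget component, then removes itself.
; On BeginPlay it writes DamageAmount into the widget's text and tints it by hit type, with crit color taking priority over magic, then the default.
; A timeline then drives a per-update local Z offset to move the actor and destroys it when finished.
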(event `self.ReceiveBeginPlay`
  (bind _aswbp_damage_text (cast `/Game/WBP_DamageText` (`WidgetComponent.GetUserWidgetObject` (`self.DamageWidget`))))
  (`TextBlock.SetText` (`/Game/WBP_DamageText.DamageText` _aswbp_damage_text) (`KismetTextLibrary.Conv_DoubleToText` (`self.DamageAmount`) "HalfToEven"))
  (`UserWidget.SetColorAndOpacity` _aswbp_damage_text (select `bool` (`self.IsCrit`) :`false` (select `bool` (`self.IsMagic`) :`false` (struct :`R` 1.0 :`G` 0.762115 :`B` 0.161458 :`A` 1.0) :`true` (struct :`R` 0.521667 :`G` 0.075151 :`B` 0.744792 :`A` 1.0) :!type "LinearColor Structure") :`true` (struct :`R` 1.0 :`G` 0.104167 :`B` 0.104167 :`A` 1.0)))
  (bind (_direction _z_offset) (`Timeline|Timeline` :!via `PlayFromStart`)
    (:`Update`
      (`self.K2_AddActorLocalOffset` (`KismetMathLibrary.MakeVector` 0.0 0.0 _z_offset)))
    (:`Finished`
      (`self.K2_DestroyActor`))))

(fn `UserConstructionScript`)